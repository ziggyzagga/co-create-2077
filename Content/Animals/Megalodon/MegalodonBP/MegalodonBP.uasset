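; Megalodon creature Blueprint that wanders between arrow markers and goes after players who come near.
; A looping timer, with its interval randomized at BeginPlay, picks a random arrow, then timelines lerp the mesh's yaw-corrected rotation and position toward it.
; Player overlap with the detection radius runs AIMoveTo on that actor and plays a bite montage on success.
; Exit only resets ChaseActor; Attack and Chase functions are empty stubs.
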(event `self.ReceiveBeginPlay`
  (`KismetSystemLibrary.K2_SetTimerDelegate` (delegate `SwimAround`) (`KismetMathLibrary.RandomFloatInRange` 3.0 7.0) true))

(event `SwimAround`
  (`self.FindNextLocationAndRotation`)
  (`self.RotateMesh`)
  (`self.MoveToLocation`))

(event `FindNextLocationAndRotation`
  (bind (_returnvalue_x _returnvalue_y _returnvalue_z) (`KismetMathLibrary.BreakVector` (`SceneComponent.K2_GetComponentLocation` (`self.Mesh`))))
  (bind _array (`|MakeArray` (`self.Arrow1`) (`self.Arrow2`) (`self.Arrow3`) (`self.Arrow4`) (`self.Arrow5`) (`self.Arrow6`) (`self.Arrow7`) (`self.Arrow8`) (`self.Arrow9`)))
  (bind (_returnvalue_roll _returnvalue_pitch _returnvalue_yaw) (`KismetMathLibrary.BreakRotator` (`KismetMathLibrary.FindLookAtRotation` (`KismetMathLibrary.MakeVector` _returnvalue_x _returnvalue_y _returnvalue_z) (`self.TargetLocation`))))
  (set `self.TargetLocation` (`SceneComponent.K2_GetComponentLocation` (`|GetArrayItem` _array (`KismetMathLibrary.RandomIntegerInRange` 0 (`KismetArrayLibrary.Array_LastIndex` _array)))))
  (set `self.NextRotation` (`KismetMathLibrary.MakeRotator` _returnvalue_roll _returnvalue_pitch (- _returnvalue_yaw 90.0))))

(event `RotateMesh`
  (bind _mesh (`self.Mesh`))
  (bind (_direction _rotateft) (`Timeline|Timeline` :!via `PlayFromStart`)
    (:`Update`
      (`SceneComponent.K2_SetWorldRotation` _mesh (`KismetMathLibrary.RLerp` (`SceneComponent.K2_GetComponentRotation` _mesh) (`self.NextRotation`) _rotateft) false false))))

(event `MoveToLocation`
  (bind _mesh (`self.Mesh`))
  (bind (_direction _swimft) (`Timeline|MoveSwimTL` :!via `PlayFromStart`)
    (:`Update`
      (`SceneComponent.K2_SetWorldLocation` _mesh (`KismetMathLibrary.VLerp` (`SceneComponent.K2_GetComponentLocation` _mesh) (`self.TargetLocation`) _swimft) false false))))

(event `self.RadiusPlayerDetect.OnComponentBeginOverlap`
  (params (OverlappedComponent :type "PrimitiveComponent Object Reference") (OtherActor :type "Actor Object Reference") (OtherComp :type "PrimitiveComponent Object Reference") (OtherBodyIndex :type Integer) (bFromSweep :type Boolean) (SweepResult :type "HitResult Structure (by ref)"))
  (if (`self.ActorHasTag` OtherActor "Player")
    (bind _output_get (set `self.ChaseActor` OtherActor))
    (`|AIMoveTo` self (0.0 0.0 0.0) _output_get
      (:`OnSuccess`
        (`|PlayMontage` null "/Game/Animals/Megalodon/Mesh/megalodon/SkeletalMeshes/bite_Montage.bite_Montage")))))

(event `self.RadiusPlayerDetect.OnComponentEndOverlap`
  (params (OverlappedComponent :type "PrimitiveComponent Object Reference") (OtherActor :type "Actor Object Reference") (OtherComp :type "PrimitiveComponent Object Reference") (OtherBodyIndex :type Integer))
  (if (`self.ActorHasTag` OtherActor "Player")
    (set `self.ChaseActor` self)))

(fn `Attack`)

(fn `Chase`
  (params (ChaseActor :type "Actor Object Reference")))

(fn `UserConstructionScript`)