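; Fox animal Blueprint that wanders the level on its own.
; A looping timer, with its interval randomized once at BeginPlay, picks a nearby reachable point, issues an AI MoveTo and immediately snaps the fox's yaw toward it.
; Tick sets the Stopped flag from movement velocity, inverted relative to its name: true while moving, false when still.
; Despite the WalkAndEat event name, no eating logic is present.
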(event `self.ReceiveBeginPlay`
  (`KismetSystemLibrary.K2_SetTimerDelegate` (delegate `WalkAndEat\\`) (`KismetMathLibrary.RandomFloatInRange` 2.0 5.0) true))

(event `WalkAndEat\\`
  (bind _returnvalue (`self.K2_GetActorLocation`))
  (bind (_returnvalue_roll _returnvalue_pitch) (`KismetMathLibrary.BreakRotator` (`self.K2_GetActorRotation`)))
  (bind (_returnvalue_roll_2 _returnvalue_pitch_2 _returnvalue_yaw) (`KismetMathLibrary.BreakRotator` (`KismetMathLibrary.FindLookAtRotation` _returnvalue (`self.Random Location`))))
  (bind _output_get (set `self.Random Location` (`NavigationSystemV1.K2_GetRandomReachablePointInRadius` _returnvalue 500.0 null null)))
  (`|AIMoveTo` self _output_get null
    (:`then`
      (`self.K2_SetActorRotation` (`KismetMathLibrary.MakeRotator` _returnvalue_roll_2 _returnvalue_pitch _returnvalue_yaw)))))

(event `self.ReceiveTick`
  (params (DeltaSeconds :type "Float (single-precision)"))
  (if (> (`KismetMathLibrary.VSize` (`MovementComponent.Velocity` (`self.CharacterMovement`))) 0.0)
    (set `self.Stopped?` true)
    (else
      (set `self.Stopped?` false))))

(fn `UserConstructionScript`)