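; First-person player character for a litter-collecting game with swimming, capacity-limited pickups, money earned from held litter and shop item ownership.
; Ocean overlap counting toggles swimming; a one-second timer updates stamina and underwater oxygen, with empty oxygen lerping the player to spawn.
; Tick checks camera submersion, plays head-bob shakes and line-traces for BPI_Interact actors, driving crosshair and input messages.
; Collected actors shrink toward the player before being destroyed.
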(event `StartSwim`
  (bind _charactermovement (`self.CharacterMovement`))
  ; StartAndStopSwimming
  (set `PhysicsVolume.bWaterVolume` true (`MovementComponent.GetPhysicsVolume` _charactermovement))
  (`CharacterMovementComponent.SetMovementMode` _charactermovement "MOVE_Swimming" 0)
  (set `self.Swim?` true))

(event `self.ReceiveTick`
  (params (DeltaSeconds :type "Float (single-precision)"))
  (bind (_returnvalue_x _returnvalue_y _returnvalue_z) (`KismetMathLibrary.BreakVector` (`SceneComponent.K2_GetComponentLocation` (`self.FirstPersonCamera`))))
  (bind (_returnvalue_x_2 _returnvalue_y_2 _returnvalue_z_2) (`KismetMathLibrary.BreakVector` (`self.K2_GetActorLocation` (`self.Water`))))
  ; Oxygen + Widget + HeadBob
  (`|ExecutionSequence`
    (:`then_0`
      (if (`self.Swim?`)
        (if (< _returnvalue_z _returnvalue_z_2)
          (set `self.UnderWater?` true)
          (else
            (set `self.UnderWater?` false)))
        (elif (`self.CanHeadBOB?`)
          (`self.HeadBoBEvent`))))
    (:`then_1`
      (`self.Event Project Interaction Line Trace`))))

(event `LaunchAtSpawnPoint`
  ; LaunchAtSpawnPoint
  (bind (_direction _launchfloat) (`Timeline|Launch` :!via `PlayFromStart`)
    (:`Update`
      (bind (_returnvalue_x _returnvalue_y _returnvalue_z) (`KismetMathLibrary.BreakVector` (`KismetMathLibrary.VLerp` (`self.K2_GetActorLocation`) (`self.SpawnPoint`) _launchfloat)))
      (`self.K2_SetActorLocation` (`KismetMathLibrary.MakeVector` _returnvalue_x _returnvalue_y (+ _returnvalue_z 90.0))))))

(event `ActorCollectedAnim`
  ; CollectedActorAnim
  (`|ExecutionSequence`
    (:`then_0`
      (bind (_direction _scalemoveft) (`Timeline|ActorScaleAndMoveTL` :!via `PlayFromStart`)
        (:`Update`
          (bind _last_interactable_actor (`self.Last Interactable Actor`)
            (:`then`
              (`|ExecutionSequence`
                (:`then_0`
                  (`self.SetActorRelativeScale3D` _last_interactable_actor (`KismetMathLibrary.VLerp` (`self.GetActorRelativeScale3D` _last_interactable_actor) (0.3 0.3 0.3) _scalemoveft)))
                (:`then_1`
                  (`self.K2_SetActorLocation` _last_interactable_actor (`KismetMathLibrary.VLerp` (`self.K2_GetActorLocation` _last_interactable_actor) (+ (`self.K2_GetActorLocation`) (0.0 0.0 30.0)) _scalemoveft) false false))))
            (:`else`)))))
    (:`then_1`
      (`self.SetActorEnableCollision` _last_interactable_actor false)
      (`KismetSystemLibrary.Delay` 0.5)
      (`self.K2_DestroyActor` _last_interactable_actor))))

(event `StopSwim`
  (bind _charactermovement (`self.CharacterMovement`))
  ; StartAndStopSwimming
  (set `PhysicsVolume.bWaterVolume` false (`MovementComponent.GetPhysicsVolume` _charactermovement))
  (`CharacterMovementComponent.SetMovementMode` _charactermovement "MOVE_Walking" 0)
  (set `self.Swim?` false))

(event `self.ReceiveBeginPlay`
  ; Oxygen + Widget + HeadBob
  (`KismetSystemLibrary.K2_SetTimerDelegate` (delegate `UpdateOxygen`) 1.0 true))

(event `self.ReceivePossessed`
  (params (NewController :type "Controller Object Reference"))
  ; Oxygen + Widget + HeadBob
  (set `self.CanHeadBOB?` true))

(event `self.ReceiveUnpossessed`
  (params (OldController :type "Controller Object Reference"))
  ; Oxygen + Widget + HeadBob
  (set `self.CanHeadBOB?` false))

(event `self.WaterCheck.OnComponentBeginOverlap`
  (params (OverlappedComponent :type "PrimitiveComponent Object Reference") (OtherActor :type "Actor Object Reference") (OtherComp :type "PrimitiveComponent Object Reference") (OtherBodyIndex :type Integer) (bFromSweep :type Boolean) (SweepResult :type "HitResult Structure (by ref)"))
  ; WaterControl
  (bind _aswater_body_ocean_blueprint (cast `/Game/Map/WaterBodyBP/WaterBodyOcean_Blueprint` OtherActor))
  (set `self.Water` _aswater_body_ocean_blueprint)
  (set `self.WaterOverlapCount` (+ (`self.WaterOverlapCount`) 1))
  (`self.StartSwim`))

(event `UpdateStamina`
  (bind _stamina (`self.Stamina`))
  ; Stamina
  (if (`self.Swim?`)
    (bind _output_get (set `self.Stamina` (- _stamina (`self.StaminaDrain`))))
    (if (<= _output_get 0.0)
      (`self.LaunchCharacter` (0.0 0.0 50.0)))
    (else
      (set `self.Stamina` (`KismetMathLibrary.FClamp` (+ _stamina (`self.StaminaRecovery`)) 0.0 (`self.MaxStamina`))))))

(event `UpdateOxygen`
  (bind _oxygen (`self.Oxygen`))
  ; Oxygen + Widget + HeadBob
  (`self.UpdateStamina`)
  (if (and (`self.Swim?`) (`self.UnderWater?`))
    (bind _output_get (set `self.Oxygen` (- _oxygen (`self.OxygenDrain`))))
    (if (<= _output_get 0.0)
      (`self.LaunchAtSpawnPoint`))
    (else
      (set `self.Oxygen` (`KismetMathLibrary.FClamp` (+ _oxygen (`self.OxygenRecover`)) 0.0 (`self.MaxOxygen`))))))

(event `self.WaterCheck.OnComponentEndOverlap`
  (params (OverlappedComponent :type "PrimitiveComponent Object Reference") (OtherActor :type "Actor Object Reference") (OtherComp :type "PrimitiveComponent Object Reference") (OtherBodyIndex :type Integer))
  ; WaterControl
  (cast `/Game/Map/WaterBodyBP/WaterBodyOcean_Blueprint` OtherActor)
  (bind _output_get (set `self.WaterOverlapCount` (- (`self.WaterOverlapCount`) 1)))
  (if (<= _output_get 0)
    (`self.StopSwim`)))

(event `HeadBobEvent`
  ; Oxygen + Widget + HeadBob
  (`self.HeadBob`))

(event `Event Project Interaction Line Trace`
  (bind _hud_widget (`self.HUD Widget`))
  (bind _returnvalue (`SceneComponent.K2_GetComponentLocation` (`self.FirstPersonCamera`)))
  ; Interaction Logic
  (if (`self.Allow Interaction`)
    (bind _outhit (`KismetSystemLibrary.LineTraceSingle` _returnvalue (+ _returnvalue (* (`SceneComponent.GetForwardVector` (`self.FirstPersonCamera`)) (`self.Interaction Range`))) "TraceTypeQuery1"))
    (bind _output_get (set `self.Interaction Hit Result` _outhit))
    (bind (_bblockinghit _binitialoverlap _time _distance _location _impactpoint _normal _impactnormal _physmat _hitactor) (`GameplayStatics.BreakHitResult` _output_get))
    (`|ExecutionSequence`
      (:`then_0`
        (set `self.Interaction Blocking Hit` _bblockinghit))
      (:`then_1`
        (set `self.Interaction Impact Point` _impactpoint))
      (:`then_2`
        (set `self.Interaction Hit Actor` _hitactor))
      (:`then_3`
        (if (`self.Interaction Blocking Hit`)
          (bind _returnvalue_2 (`KismetSystemLibrary.DoesImplementInterface` (`self.Interaction Hit Actor`) "/Game/Blueprints/Interactables/BPI_Interact.BPI_Interact_C"))
          (if _returnvalue_2
            (bind _last_interactable_actor (`self.Last Interactable Actor`)
              (:`then`
                (if (== _last_interactable_actor (`self.Interaction Hit Actor`))
                  (set `self.Last Interactable Actor` (`self.Interaction Hit Actor`) :!label _label)
                  (else
                    (message `/Game/Blueprints/Interactables/BPI_Interact.LookedAt` (`self.Last Interactable Actor`) false)
                    (set `self.Last Interactable Actor` (`self.Interaction Hit Actor`)))))
              (:`else`
                (goto _label)))
            (bind _hideinteraction (message `/Game/Blueprints/Interactables/BPI_Interact.LookedAt` (`self.Last Interactable Actor`) true))
            (if _hideinteraction
              (`/Game/Blueprints/Widgets/WBP_HumanHUD.HideDotCrosshair` _hud_widget)
              (else
                (`/Game/Blueprints/Widgets/WBP_HumanHUD.ShowCircleCrosshair` _hud_widget)))
            (else
              (`self.InteractingActorLost`)))
          (else
            (`self.InteractingActorLost`)))))
    (else
      (`self.InteractingActorLost`))))

(event `EnhancedInput|/Game/Characters/Input/IA_Interact`
  (params (ActionValue :type Boolean) (ElapsedSeconds :type "Float (double-precision)") (TriggeredSeconds :type "Float (double-precision)") (InputAction :type "InputAction Object Reference" :default "/Game/Characters/Input/IA_Interact.IA_Interact"))
  ; Interaction Logic
  (:`Started`
    (bind _last_interactable_actor (`self.Last Interactable Actor`)
      (:`then`
        (message `/Game/Blueprints/Interactables/BPI_Interact.InteractStart` _last_interactable_actor))
      (:`else`)))
  (:`Canceled`
    (bind _last_interactable_actor_2 (`self.Last Interactable Actor` :!label _label_2)
      (:`then`
        (message `/Game/Blueprints/Interactables/BPI_Interact.InteractEnd` _last_interactable_actor_2))
      (:`else`)))
  (:`Completed`
    (goto _label_2)))

(fn `AttemptCollectLitter`
  (params (InLitterValue :type Integer))
  (locals (LitterValue :type Integer) (ProjectedHeldLitter :type Integer))
  (bind _output_get (set `local.LitterValue` InLitterValue))
  (bind _output_get_2 (set `local.ProjectedHeldLitter` (+ _output_get (`self.CurrentlyHeldLitter`))))
  (if (<= _output_get_2 (`self.MaxLitterCapacity`))
    (set `self.CurrentlyHeldLitter` (`local.ProjectedHeldLitter`))
    (`/Game/Blueprints/Widgets/WBP_HumanHUD.UpdateLitterDisplay` (`self.HUD Widget`))
    (`self.Litter Collected Signal`)
    (`self.Last Interactable Actor`
      (:`then`
        (`self.ActorCollectedAnim`)
        (return))
      (:`else`))
    (else
      (`self.Litter Rejected Signal`))))

(fn `GiveMoney`
  (bind _hud_widget (`self.HUD Widget`))
  (set `self.Money` (+ (`self.Money`) (* (`self.CurrentlyHeldLitter`) 3)))
  (set `self.CurrentlyHeldLitter` 0)
  (`/Game/Blueprints/Widgets/WBP_HumanHUD.UpdateLitterDisplay` _hud_widget)
  (`/Game/Blueprints/Widgets/WBP_HumanHUD.UpdateMoneyDisplay` _hud_widget)
  (return))

(fn `HeadBob`
  (if (and (> (`KismetMathLibrary.VSize` (`self.GetVelocity`)) 0.0) (`self.CanJump`))
    (if true
      (`PlayerController.ClientStartCameraShake` :`self` (`GameplayStatics.GetPlayerController` 0) :`Shake` "/Game/Characters/LifeHuman/CameraShake/CameraSRun.CameraSRun_C")
      (return))
    (else
      (`PlayerController.ClientStartCameraShake` :`self` (`GameplayStatics.GetPlayerController` 0) :`Shake` "/Game/Characters/LifeHuman/CameraShake/CameraSidle.CameraSidle_C")
      (return))))

(fn `InteractingActorLost`
  (`/Game/Blueprints/Widgets/WBP_HumanHUD.HideCircleCrosshair` (`self.HUD Widget`))
  (bind _last_interactable_actor (`self.Last Interactable Actor`)
    (:`then`
      (message `/Game/Blueprints/Interactables/BPI_Interact.LookedAt` _last_interactable_actor false)
      (return))
    (:`else`)))

(fn `LoseMoney`
  (params (MoneyToLose :type Integer))
  (locals (`Money To Lose` :type Integer))
  (set `local.Money To Lose` MoneyToLose)
  (set `self.Money` (- (`self.Money`) (`local.Money To Lose`))))

(fn `SetItemOwnership`
  (params (InItem :type "/Game/Blueprints/Shopping/E_ShopItems Enum" :default "NewEnumerator0") (InOwnership :type Boolean))
  (locals (Item :type "/Game/Blueprints/Shopping/E_ShopItems Enum" :default "NewEnumerator0") (Ownership :type Boolean))
  (`|ExecutionSequence`
    (:`then_0`
      (set `local.Item` InItem))
    (:`then_1`
      (set `local.Ownership` InOwnership))
    (:`then_2`
      (`BlueprintMapLibrary.Map_Add` (`self.Shop Items Ownership`) (`local.Item`) (`local.Ownership`)))))

(fn `UserConstructionScript`
  (`parent.UserConstructionScript`))