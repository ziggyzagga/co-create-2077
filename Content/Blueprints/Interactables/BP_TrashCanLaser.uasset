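; BP_TrashCanLaser is an interactable that pays the player money when interacted with while looked at.
; On BeginPlay it caches the player's BP_LifeHuman and binds to its litter collected and rejected signals.
; LookedAt sets the gaze flag that gates all responses: collection sets IsCollected, rejection does nothing, and the payout ignores IsCollected.
; A PlaySoundByIndex helper sets an integer audio parameter before playing, but is not called here.
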(event `self.ReceiveBeginPlay`
  (bind _asbp_life_human (cast `/Game/Characters/LifeHuman/BP_LifeHuman` (`GameplayStatics.GetPlayerCharacter` 0)))
  (set `self.PlayerHuman` _asbp_life_human)
  (`|ExecutionSequence`
    (:`then_0`
      (add `/Game/Characters/LifeHuman/BP_LifeHuman.Litter Collected Signal` (`self.PlayerHuman`) (delegate `Collected`)))
    (:`then_1`
      (add `/Game/Characters/LifeHuman/BP_LifeHuman.Litter Rejected Signal` (`self.PlayerHuman`) (delegate `Rejected`)))))

(event `Collected`
  (if (and (`self.IsLookedAt`) (not (`self.IsCollected`)))
    (set `self.IsCollected` true)))

(event `self.InteractStart`
  (if (`self.IsLookedAt`)
    (`/Game/Characters/LifeHuman/BP_LifeHuman.GiveMoney` (`self.PlayerHuman`))))

(event `Rejected`
  (if (`self.IsLookedAt`)
    _))

(fn `LookedAt`
  (params (inLookedAt :type Boolean))
  (returns (HideInteraction :type Boolean))
  (set `self.IsLookedAt` inLookedAt)
  (return (`self.HideInteraction`)))

(fn `PlaySoundByIndex`
  (params (InIndexName :type Name) (InIndex :type Integer) (InStartTime :type "Float (double-precision)"))
  (bind _audiocomponent (`self.AudioComponent`))
  (`|ExecutionSequence`
    (:`then_0`
      (`AudioComponent.SetIntParameter` _audiocomponent InIndexName InIndex))
    (:`then_1`
      (`AudioComponent.Play` _audiocomponent InStartTime))))

(fn `UserConstructionScript`)